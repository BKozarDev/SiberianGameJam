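; Player character with mouse-aimed primary and secondary melee combos, a cooldown-gated dodge roll, interaction and health.
; Attacks cycle montages from per-type maps, whose damage and range feed the attack action component and Niagara slash effects.
; The dodge cancels montages and moves by timeline, toggling capsule collision for i-frames.
; Damage drains the health component; death spawns a mesh-based Niagara effect, then loads MainMap.
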(event Custom|DodgeRoll
  (bind _capsulecomponent (Variables|Collision|GetCapsuleComponent))
  (bind _mesh (Variables|Character|GetMesh))
  (bind _returnvalue (Components|SkeletalMesh|GetAnimInstance _mesh))
  (Utilities|FlowControl|Gate false :!label _label
    (:Exit
      (Utilities|FlowControl|Sequence
        (:then_0
          (Variables|/Script/Engine.CharacterMovementComponent|SetMaxWalkSpeed (Variables|Character|GetCharacterMovement) 0.0)
          (Variables|PlayerCharacter|SetIsDodgeRolling true)
          (Animation|Montage|MontageStop _returnvalue 0.0 (Animation|Montage|GetCurrentActiveMontage _returnvalue))
          (Variables|Default|SetDodgeRollDelta (* (Variables|PlayerCharacter|GetDodgeRollForce) (Math|Vector|SelectVector (Math|Conversions|ToVector(Vector2D) (Input|EnhancedActionValues|GetIA_PlayerMove)) (Transformation|GetActorForwardVector) (> (Math|Vector|VectorLength (Math|Conversions|ToVector(Vector2D) (Input|EnhancedActionValues|GetIA_PlayerMove))) 0.01))))
          (Variables|PlayerCharacter|SetIsAttacking false)
          (Audio|PlaySound2D "/Game/LopataProject/Sounds/SC_Dash.SC_Dash" 1.0 1.0 0.0 0 0)
          (bind _forcemp (Timeline|TL_DodgeRoll PlayFromStart)
            (:Update
              (Transformation|AddActorWorldOffset (* (Variables|Default|GetDodgeRollDelta) _forcemp) true))
            (:Finished
              (Variables|/Script/Engine.CharacterMovementComponent|SetMaxWalkSpeed (Variables|Character|GetCharacterMovement) (Variables|PlayerCharacter|GetMaxMoveSpeed))
              (Variables|PlayerCharacter|SetIsDodgeRolling false)
              (Variables|PlayerCharacter|SetCheckNextHit true))
            (:ToggleIFrames
              (Utilities|FlowControl|FlipFlop
                (:A
                  (Collision|SetCollisionResponsetoChannel _capsulecomponent "ECC_GameTraceChannel2" "ECR_Ignore")
                  (Collision|SetCollisionResponsetoChannel _capsulecomponent "ECC_Pawn" "ECR_Ignore"))
                (:B
                  (Collision|SetCollisionResponsetoChannel _capsulecomponent "ECC_GameTraceChannel2" "ECR_Overlap")
                  (Collision|SetCollisionResponsetoChannel _capsulecomponent "ECC_Pawn" "ECR_Block"))))))
        (:then_1
          (goto _label Close))
        (:then_2
          (Utilities|Time|SetTimerbyEvent (delegate Custom|DodgeRollReady) (Variables|PlayerCharacter|GetDodgeRollCooldown)))))))

(event Custom|DodgeRollReady
  (bind _capsulecomponent (Variables|Collision|GetCapsuleComponent))
  (bind _mesh (Variables|Character|GetMesh))
  (bind _returnvalue (Components|SkeletalMesh|GetAnimInstance _mesh))
  (Utilities|FlowControl|Sequence
    (:then_0
      (Utilities|FlowControl|Gate false) ; enters at Open
    )))

(event Custom|AttackPrimary
  (bind _returnvalue (Transformation|GetActorLocation))
  (if (not (Variables|PlayerCharacter|GetIsAttacking))
    (if (Variables|Default|GetIsPrimaryAttack)
      _
      (else
        (Variables|PlayerCharacter|SetAttackIndex -1)
        (Variables|Default|SetIsPrimaryAttack true)))
    (Variables|PlayerCharacter|SetIsAttacking true)
    (Variables|/Script/Engine.CharacterMovementComponent|SetMaxWalkSpeed (Variables|Character|GetCharacterMovement) 0.0)
    (bind _location (Utilities|GetMouseWorldPosition)
      (:Return
        (Transformation|SetActorRotation (Math|Rotator|FindLookatRotation (Math|Vector|MakeVector (.x _returnvalue) (.y _returnvalue) 0.0) (Math|Vector|MakeVector (.x _location) (.y _location) 0.0)) true)
        (Physics|AddImpulse (Variables|Character|GetCharacterMovement) (* (Transformation|GetActorForwardVector) (Variables|Default|GetAttackImpulse)) true)
        (Math|Integer|IncrementInt (Variables|PlayerCharacter|GetAttackIndex)
          (:%20%20
            (if (> (Variables|PlayerCharacter|GetAttackIndex) (- (Utilities|Map|Length (Variables|PlayerCharacter|GetAttackPrimaryMoves)) 1))
              (Variables|PlayerCharacter|SetAttackIndex 0))
            (bind _keys (Utilities|Map|Keys (Variables|PlayerCharacter|GetAttackPrimaryMoves)))
            (bind _output_get (Variables|PlayerCharacter|SetCurrentAttack (Utilities|Array|Get(acopy) _keys (Variables|PlayerCharacter|GetAttackIndex))))
            (Animation|Montage|PlayMontage (Variables|Character|GetMesh) _output_get
              (:OnInterrupted
                (Utilities|FlowControl|RetriggerableDelay 1.2)
                (Variables|PlayerCharacter|SetAttackIndex -1)
                (Variables|PlayerCharacter|SetIsAttacking false)
                (Variables|PlayerCharacter|SetCurrentAttack 0)
                (Variables|Default|SetIsPrimaryAttack false)))))))))

(event Custom|Interact
  (Default|Interact (Variables|Default|GetBPAC_InteractionQueue)))

(event Custom|AttackSecondary
  (bind _returnvalue (Transformation|GetActorLocation))
  (if (not (Variables|PlayerCharacter|GetIsAttacking))
    (if (Variables|Default|GetIsPrimaryAttack)
      (Variables|PlayerCharacter|SetAttackIndex -1))
    (Variables|PlayerCharacter|SetIsAttacking true)
    (Variables|Default|SetIsPrimaryAttack false)
    (Variables|/Script/Engine.CharacterMovementComponent|SetMaxWalkSpeed (Variables|Character|GetCharacterMovement) 0.0)
    (bind _location (Utilities|GetMouseWorldPosition)
      (:Return
        (Transformation|SetActorRotation (Math|Rotator|FindLookatRotation (Math|Vector|MakeVector (.x _returnvalue) (.y _returnvalue) 0.0) (Math|Vector|MakeVector (.x _location) (.y _location) 0.0)) true)
        (Physics|AddImpulse (Variables|Character|GetCharacterMovement) (* (Transformation|GetActorForwardVector) (Variables|Default|GetAttackImpulse)) true)
        (Math|Integer|IncrementInt (Variables|PlayerCharacter|GetAttackIndex)
          (:%20%20
            (if (> (Variables|PlayerCharacter|GetAttackIndex) (- (Utilities|Map|Length (Variables|PlayerCharacter|GetAttackSecondaryMoves)) 1))
              (Variables|PlayerCharacter|SetAttackIndex 0))
            (bind _keys (Utilities|Map|Keys (Variables|PlayerCharacter|GetAttackSecondaryMoves)))
            (bind _output_get (Variables|PlayerCharacter|SetCurrentAttack (Utilities|Array|Get(acopy) _keys (Variables|PlayerCharacter|GetAttackIndex))))
            (Animation|Montage|PlayMontage (Variables|Character|GetMesh) _output_get
              (:OnInterrupted
                (Utilities|FlowControl|RetriggerableDelay 1.2)
                (Variables|PlayerCharacter|SetAttackIndex -1)
                (Variables|PlayerCharacter|SetIsAttacking false)
                (Variables|PlayerCharacter|SetCurrentAttack 0)))))))))

(event Custom|Dead
  (bind _returnvalue (Transformation|GetActorTransform))
  (Audio|PlaySound2D "/Game/LopataProject/Sounds/SC_Death.SC_Death" 1.0 1.0 0.0 0 0)
  (bind _returnvalue_2 (Class|NiagaraFunctionLibrary|SpawnSystematLocationwithParams (Utilities|Struct|MakeFXSystemSpawnParameters self "/Game/LopataProject/Common/FX/NS_MeshDeathEffect.NS_MeshDeathEffect" (.location _returnvalue) (.rotation _returnvalue) "1.000000,1.000000,1.000000" 0 "None" "KeepWorldPosition" true true)))
  (Class|NiagaraFunctionLibrary|OverrideSystemUserVariableSkeletalMeshComponent _returnvalue_2 "SkelMesh" (Variables|Character|GetMesh))
  (Class|NiagaraComponent|SetVariableInt _returnvalue_2 "ParticleCount" 200)
  (Rendering|SetActorHiddenInGame true)
  (Collision|SetActorEnableCollision false)
  (Utilities|FlowControl|Delay 3.0)
  (Game|OpenLevel(byName) "MainMap"))

(event Custom|TeleportPlayer
  (params (NewLocation :type Vector))
  (Variables|/Script/Engine.SpringArmComponent|SetbEnableCameraLag (Variables|Default|GetSpringArm) false)
  (Transformation|SetActorLocation NewLocation false true)
  (Utilities|FlowControl|Delay 0.2)
  (Variables|/Script/Engine.SpringArmComponent|SetbEnableCameraLag (Variables|Default|GetSpringArm) true))

(event Game|Damage|EventAnyDamage
  (params (Damage :type Float%20%28single-precision%29) (DamageType :type Damage%20Type%20Object%20Reference) (InstigatedBy :type Controller%20Object%20Reference) (DamageCauser :type Actor%20Object%20Reference))
  (Default|DecreaseValue (Variables|Default|GetBPAC_HealthComponent) (Math|Float|Truncate Damage)))

(event EventBeginPlay
  (|CallParentFunction)
  (Variables|PlayerCharacter|SetCheckNextHit true)
  (EventDispatchers|BindEventtoOnValueZero (Variables|Default|GetBPAC_HealthComponent) (EventDispatchers|CreateEvent :!event Custom|Dead)))

(event EventTick
  (params (DeltaSeconds :type Float%20%28single-precision%29))
  (bind _charactermovement (Variables|Character|GetCharacterMovement))
  (bind _velocity (Variables|/Script/Engine.MovementComponent|GetVelocity _charactermovement))
  (bind (_x _y) (Math|Vector|BreakVector _velocity))
  (|CallParentFunction DeltaSeconds)
  (if (not (Variables|PlayerCharacter|GetIsAttacking))
    (if (and (> (Math|Vector|VectorLength _velocity) 0.01) (not (Variables|PlayerCharacter|GetIsDodgeRolling)))
      (Transformation|SetActorRotation (Math|Rotator|MakeRotfromXZ (Math|Vector|Normalize (Math|Vector|MakeVector _x _y 0.0)) (Math|Vector|MakeVector 0.0 0.0 1.0)) true))))

(event Input|KeyboardEvents|H
  (params (Key :type Key%20Structure :default "None"))
  (:Pressed
    (Default|DecreaseValue (Variables|Default|GetBPAC_HealthComponent) 5)))

(fn ConstructionScript
  (Variables|/Script/Engine.CharacterMovementComponent|SetMaxWalkSpeed (Variables|Character|GetCharacterMovement) (Variables|PlayerCharacter|GetMaxMoveSpeed))
  (Components|Timeline|SetPlayRate (Variables|Default|GetTL_DodgeRoll) (/ 1.0 (Variables|PlayerCharacter|GetDodgeRollDuration))))

(fn DoAttackAction
  (params (AttackingActor :type Actor%20Object%20Reference))
  (bind (_params _isfound) (CallFunction|GetCurrentAttackParams))
  (bind _asbp_enemy_base (Utilities|Casting|CastToBP_EnemyBase AttackingActor))
  (Variables|PlayerCharacter|GetCurrentAttack
    (:then
      (if _isfound
        (Default|StartAction (Variables|Default|GetBPAC_AttackingAction) _asbp_enemy_base (Utilities|Array|MakeArray (Utilities|String|ToString(Float) (Utilities|Struct|BreakS_AttackParam _params))))
        (else
          (Default|StartAction (Variables|Default|GetBPAC_AttackingAction) _asbp_enemy_base (Utilities|Array|MakeArray "") :!label _label))))
    (:else
      (goto _label)))
  (Audio|PlaySound2D "/Game/LopataProject/Sounds/SC_Hit.SC_Hit" 1.0 1.0 0.0 0 0))

(fn RefreshAttackState
  (Variables|PlayerCharacter|SetIsAttacking false)
  (Variables|PlayerCharacter|SetCheckNextHit true)
  (Variables|PlayerCharacter|SetAttackIndex 0))

(fn GetCurrentAttackParams
  (bind _attacksecondarymoves (Variables|PlayerCharacter|GetAttackSecondaryMoves))
  (bind _currentattack (Variables|PlayerCharacter|GetCurrentAttack))
  (bind _attackprimarymoves (Variables|PlayerCharacter|GetAttackPrimaryMoves))
  (bind _currentattack_2 (Variables|PlayerCharacter|GetCurrentAttack))
  (bind (_value _returnvalue) (Utilities|Map|Find _attacksecondarymoves _currentattack))
  (bind (_value_2 _returnvalue_2) (Utilities|Map|Find _attackprimarymoves _currentattack_2))
  (if (Variables|Default|GetIsPrimaryAttack)
    (return _value_2 _returnvalue_2)
    (else
      (return _value _returnvalue))))

(fn PlayPrimaryFXbyIndex
  (params (AttackIndex :type Integer))
  (bind _returnvalue (Transformation|GetActorTransform))
  (bind _returnvalue_2 (Transformation|GetActorTransform))
  (bind _returnvalue_3 (Transformation|GetActorTransform))
  (bind _isprimaryattack (Variables|Default|GetIsPrimaryAttack))
  (switch int AttackIndex
    (:0
      (if _isprimaryattack
        (bind _returnvalue_4 (Class|NiagaraFunctionLibrary|SpawnSystematLocationwithParams (Utilities|Struct|MakeFXSystemSpawnParameters self "/Game/LopataProject/Player/FX/NS_PlayerHorizontalAttack.NS_PlayerHorizontalAttack" (.location _returnvalue_3) (.rotation _returnvalue_3) "1.000000,1.000000,1.000000" 0 "None" "KeepWorldPosition" true true)))
        (Class|NiagaraComponent|SetVariableBool _returnvalue_4 "Reverse" false)
        (Niagara|SetNiagaraVariable(Float) _returnvalue_4 "Radius" (.Range (Utilities|Struct|BreakS_AttackParam (.Params (CallFunction|GetCurrentAttackParams)))))
        (else
          (bind _returnvalue_5 (Class|NiagaraFunctionLibrary|SpawnSystematLocationwithParams (Utilities|Struct|MakeFXSystemSpawnParameters self "/Game/LopataProject/Player/FX/NS_PlayerForwardAttack.NS_PlayerForwardAttack" (.location _returnvalue_2) (.rotation _returnvalue_2) "1.000000,1.000000,1.000000" 0 "None" "KeepWorldPosition" true true) :!label _label))
          (Niagara|SetNiagaraVariable(Float) _returnvalue_5 "Range" (.Range (Utilities|Struct|BreakS_AttackParam (.Params (CallFunction|GetCurrentAttackParams))))))))
    (:1
      (if _isprimaryattack
        (bind _returnvalue_6 (Class|NiagaraFunctionLibrary|SpawnSystematLocationwithParams (Utilities|Struct|MakeFXSystemSpawnParameters self "/Game/LopataProject/Player/FX/NS_PlayerHorizontalAttack.NS_PlayerHorizontalAttack" (.location _returnvalue) (.rotation _returnvalue) "1.000000,1.000000,1.000000" 0 "None" "KeepWorldPosition" true true)))
        (Class|NiagaraComponent|SetVariableBool _returnvalue_6 "Reverse" true)
        (Niagara|SetNiagaraVariable(Float) _returnvalue_6 "Radius" (.Range (Utilities|Struct|BreakS_AttackParam (.Params (CallFunction|GetCurrentAttackParams)))))
        (else
          (goto _label))))))

(fn IncreaseAttack
  (params (Delta :type Float%20%28double-precision%29))
  (Variables|Default|SetAttackMultiplier (+ Delta (Variables|Default|GetAttackMultiplier)))
  (Utilities|FlowControl|Sequence
    (:then_0
      (bind _keys (Utilities|Map|Keys (Variables|PlayerCharacter|GetAttackPrimaryMoves)))
      (for _array_element _keys
        (Utilities|Map|Add (Variables|PlayerCharacter|GetAttackPrimaryMoves) _array_element (Utilities|Struct|MakeS_AttackParam (* (Variables|Default|GetAttackMultiplier) (.Damage (Utilities|Struct|BreakS_AttackParam (.Value (Utilities|Map|Find (Variables|PlayerCharacter|GetAttackPrimaryMoves) _array_element))))) (.Range (Utilities|Struct|BreakS_AttackParam (.Value (Utilities|Map|Find (Variables|PlayerCharacter|GetAttackPrimaryMoves) _array_element))))))))
    (:then_1
      (bind _keys_2 (Utilities|Map|Keys (Variables|PlayerCharacter|GetAttackSecondaryMoves)))
      (for _array_element_2 _keys_2
        (Utilities|Map|Add (Variables|PlayerCharacter|GetAttackSecondaryMoves) _array_element_2 (Utilities|Struct|MakeS_AttackParam (* (Variables|Default|GetAttackMultiplier) (.Damage (Utilities|Struct|BreakS_AttackParam (.Value (Utilities|Map|Find (Variables|PlayerCharacter|GetAttackSecondaryMoves) _array_element_2))))) (.Range (Utilities|Struct|BreakS_AttackParam (.Value (Utilities|Map|Find (Variables|PlayerCharacter|GetAttackSecondaryMoves) _array_element_2))))))))))