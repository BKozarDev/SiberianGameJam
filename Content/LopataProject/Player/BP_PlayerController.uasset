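; Player controller that translates Enhanced Input actions into commands for the controlled player pawn.
; On BeginPlay it adds the default mapping context, and movement input feeds straight into the pawn as 2D world-space movement.
; Dodge roll and primary attack cast the pawn to BP_PlayerChar and call its matching functions.
; Interact and secondary attack events are present but empty.
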(event EventBeginPlay
  (|CallParentFunction)
  (Input|AddMappingContext (PlayerController|LocalPlayerSubsystems|GetEnhancedInputLocalPlayerSubsystem) "/Game/LopataProject/Player/Input/IMC_Default.IMC_Default" 0 "(bIgnoreAllPressedKeysUntilRelease=True,bForceImmediately=False,bNotifyUserSettings=False)"))

(event Input|EnhancedActionEvents|EnhancedInputActionIA_PlayerMove
  (params (ActionValue :type Vector%202D%20Structure) (ElapsedSeconds :type Float%20%28double-precision%29) (TriggeredSeconds :type Float%20%28double-precision%29) (InputAction :type Input%20Action%20Object%20Reference :default "/Game/LopataProject/Player/Input/IA_PlayerMove.IA_PlayerMove"))
  (Pawn|Input|AddMovementInput (Pawn|GetControlledPawn) (Math|Conversions|ToVector(Vector2D) ActionValue) 1.0 false))

(event Input|EnhancedActionEvents|EnhancedInputActionIA_DodgeRoll
  (params (ActionValue :type Boolean) (ElapsedSeconds :type Float%20%28double-precision%29) (TriggeredSeconds :type Float%20%28double-precision%29) (InputAction :type Input%20Action%20Object%20Reference :default "/Game/LopataProject/Player/Input/IA_DodgeRoll.IA_DodgeRoll"))
  (bind _asbp_player_char (Utilities|Casting|CastToBP_PlayerChar (Pawn|GetControlledPawn)))
  (Default|DodgeRoll _asbp_player_char))

(event Input|EnhancedActionEvents|EnhancedInputActionIA_Interact
  (params (ActionValue :type Boolean) (ElapsedSeconds :type Float%20%28double-precision%29) (TriggeredSeconds :type Float%20%28double-precision%29) (InputAction :type Input%20Action%20Object%20Reference :default "/Game/LopataProject/Player/Input/IA_Interact.IA_Interact")))

(event Input|EnhancedActionEvents|EnhancedInputActionIA_AttackPrimary
  (params (ActionValue :type Boolean) (ElapsedSeconds :type Float%20%28double-precision%29) (TriggeredSeconds :type Float%20%28double-precision%29) (InputAction :type Input%20Action%20Object%20Reference :default "/Game/LopataProject/Player/Input/IA_AttackPrimary.IA_AttackPrimary"))
  (bind _asbp_player_char (Utilities|Casting|CastToBP_PlayerChar (Pawn|GetControlledPawn)))
  (Default|AttackPrimary _asbp_player_char))

(event Input|EnhancedActionEvents|EnhancedInputActionIA_AttackSecondary
  (params (ActionValue :type Boolean) (ElapsedSeconds :type Float%20%28double-precision%29) (TriggeredSeconds :type Float%20%28double-precision%29) (InputAction :type Input%20Action%20Object%20Reference :default "/Game/LopataProject/Player/Input/IA_AttackSecondary.IA_AttackSecondary")))

(fn ConstructionScript)