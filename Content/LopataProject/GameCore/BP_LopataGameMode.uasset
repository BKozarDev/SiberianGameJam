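; Game mode that runs level progression on MainMap, streaming levels from an ordered list as level instances spaced along X.
; Once a level is shown, it teleports the player to a PlayerStart and unloads the previous level.
; The chosen reward then joins the new level's encounter manager as an encounter.
; BindTransition hooks transitions to an event and hands each a random, non-repeating reward, except in the last two levels.
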(event Custom|PrevUnloaded
  (if (Utilities|IsValidClass (stale Custom|LoadNextLevel RewardForNextLevel))
    (bind _returnvalue (Actor|GetActorOfClass "/Game/LopataProject/Encounters/BP_EncounterManager.BP_EncounterManager_C"))
    (Utilities|Array|Add (Variables|/Game/LopataProject/Encounters/BP_EncounterManager.BP_EncounterManager_C|GetEncounters _returnvalue) (Utilities|Struct|MakeEncounterData (Utilities|Array|MakeArray (stale Custom|LoadNextLevel RewardForNextLevel))))))

(event Custom|NextLevelLoaded
  (EventDispatchers|UnbindEventfromOnLevelShown (Variables|Default|GetCurrentLevel) (delegate Custom|NextLevelLoaded))
  (Utilities|FlowControl|DelayUntilNextTick)
  (bind _returnvalue (Actor|GetActorOfClass "/Script/Engine.PlayerStart"))
  (Default|TeleportPlayer (.AsBP%20Player%20Char (Utilities|Casting|CastToBP_PlayerChar (Game|GetPlayerCharacter 0))) (Transformation|GetActorLocation _returnvalue))
  (bind _prevlevel (Variables|Default|GetPrevLevel)
    (:then
      (Variables|/Script/Engine.LevelStreaming|SetbShouldBeVisible _prevlevel false)
      (Variables|/Script/Engine.LevelStreaming|SetbShouldBeLoaded _prevlevel false)
      (EventDispatchers|BindEventtoOnLevelUnloaded _prevlevel (delegate Custom|PrevUnloaded)))
    (:else
      (if (Utilities|IsValidClass (stale Custom|LoadNextLevel RewardForNextLevel))
        (bind _returnvalue_2 (Actor|GetActorOfClass "/Game/LopataProject/Encounters/BP_EncounterManager.BP_EncounterManager_C"))
        (Utilities|Array|Add (Variables|/Game/LopataProject/Encounters/BP_EncounterManager.BP_EncounterManager_C|GetEncounters _returnvalue_2) (Utilities|Struct|MakeEncounterData (Utilities|Array|MakeArray (stale Custom|LoadNextLevel RewardForNextLevel))))))))

(event Custom|LoadNextLevel
  (params (RewardForNextLevel :type BP%20Pick%20Up%20Interaction%20Class%20Reference))
  (bind _currentlevelidx (Variables|Default|GetCurrentLevelIdx))
  (bind _levelslist (Variables|Default|GetLevelsList))
  (Math|Integer|IncrementInt (Variables|Default|GetCurrentLevelIdx)
    (:%20%20
      (if (Utilities|Array|IsValidIndex _levelslist _currentlevelidx)
        (if (< _currentlevelidx (- (Utilities|Array|LastIndex _levelslist) 1))
          (Variables|Default|SetCurrentRewardsList (Variables|Default|GetRewardsForNextLevel))
          (else
            (Variables|Default|SetCurrentRewardsList (Utilities|Array|MakeArray))))
        (Variables|Default|SetPrevLevel (Variables|Default|GetCurrentLevel))
        (bind _returnvalue (Class|LevelStreamingDynamic|LoadLevelInstancebySoftObjectPtr (Utilities|Array|Get(acopy) _levelslist _currentlevelidx) (* "5000.000000,0.000000,0.000000" (Variables|Default|GetCurrentLevelIdx)) "0, 0, 0" "" 0 false))
        (bind _output_get (Variables|Default|SetCurrentLevel _returnvalue))
        (EventDispatchers|BindEventtoOnLevelShown _output_get (delegate Custom|NextLevelLoaded))))))

(event EventBeginPlay
  (bind _returnvalue (Game|GetCurrentLevelName true))
  (if (Utilities|Enum|Equal(Enum) _returnvalue "MainMap")
    (Variables|Default|SetbAllowTransitions true)
    (Variables|Default|SetCurrentLevelIdx -1)
    (CallFunction|LoadNextLevel "/Game/LopataProject/Objects/Interaction/BP_PickUpInteraction_HealthUp.BP_PickUpInteraction_HealthUp_C")))

(fn ConstructionScript)

(fn BindTransition
  (params (Transition :type BP%20Level%20Transition%20Object%20Reference))
  (bind _currentrewardslist (Variables|Default|GetCurrentRewardsList))
  (if (Variables|Default|GetbAllowTransitions)
    (EventDispatchers|BindEventtoCallNextLevel Transition (EventDispatchers|CreateEvent :!event Custom|LoadNextLevel)) ; Unbinds automatically when triggered
    (if (Utilities|Array|IsNotEmpty (Variables|Default|GetCurrentRewardsList))
      (bind _output_get (LocalVariables|SetL_ResultReward (.OutItem (Utilities|Array|Random _currentrewardslist))))
      (Utilities|Array|RemoveItem _currentrewardslist _output_get)
      (return _output_get)
      (else
        (return 0)))))