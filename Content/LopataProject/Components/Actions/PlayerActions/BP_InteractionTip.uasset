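; BP_InteractionTip is a world-space interaction prompt that shows text through a WBP_InteractionTip widget component.
; Each tick it rotates the widget to face the first player's camera, and its construction script disables the widget's shadow casting.
; SetInteractionText forwards the given text to the underlying user widget.
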(event EventTick
  (params (DeltaSeconds :type Float%20%28single-precision%29))
  (Transformation|SetWorldRotation (Variables|Default|GetWidget) (Math|Rotator|FindLookatRotation (Transformation|GetWorldLocation (Variables|Default|GetWidget)) (Camera|GetCameraLocation (Variables|/Script/Engine.PlayerController|GetPlayerCameraManager (Game|GetPlayerController 0)))) false false))

(fn ConstructionScript
  (Rendering|SetCastShadow (Variables|Default|GetWidget) false))

(fn SetInteractionText
  (params (Text :type Text))
  (bind _aswbp_interaction_tip (Utilities|Casting|CastToWBP_InteractionTip (UserInterface|GetUserWidgetObject (Variables|Default|GetWidget))))
  (Default|SetInteractionText _aswbp_interaction_tip Text))