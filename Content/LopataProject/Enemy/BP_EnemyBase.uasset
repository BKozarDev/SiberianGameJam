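; BP_EnemyBase is the base enemy Blueprint, handling damage, attacks, death and perception filtering.
; Health component events drive the health bar and a brief retriggerable stun, while separate action components execute damage, attacks and a once-only death.
; Helpers check planar attack range and sort sensed actors by tag into follow, lost-track or ignore paths.
; Tick turns the health bar widget toward the player camera.
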(event Custom|TakingDamage
  (params (Value :type Integer))
  (Variables|Default|SetIsStunned true)
  (Utilities|FlowControl|RetriggerableDelay 0.5)
  (Variables|Default|SetIsStunned false))

(event EventBeginPlay
  (bind _bpac_healthcomponent (Variables|Default|GetBPAC_HealthComponent))
  (bind _aswbp_health_bar (Utilities|Casting|CastToWBP_HealthBar (UserInterface|GetUserWidgetObject (Variables|Default|GetWidget))))
  (Default|SetupWidget _aswbp_health_bar (Variables|Default|GetBPAC_HealthComponent))
  (EventDispatchers|BindEventtoOnValueZero _bpac_healthcomponent (EventDispatchers|CreateEvent :!event PreparetoDeath))
  (EventDispatchers|BindEventtoOnValueDecreased _bpac_healthcomponent (delegate Custom|TakingDamage))
  (Rendering|SetCastShadow (Variables|Default|GetWidget) false))

(event EventTick
  (params (DeltaSeconds :type Float%20%28single-precision%29))
  (Transformation|SetWorldRotation (Variables|Default|GetWidget) (Math|Rotator|FindLookatRotation (Transformation|GetWorldLocation (Variables|Default|GetWidget)) (Camera|GetCameraLocation (Variables|/Script/Engine.PlayerController|GetPlayerCameraManager (Game|GetPlayerController 0)))) false false))

(event Game|Damage|EventAnyDamage
  (params (Damage :type Float%20%28single-precision%29) (DamageType :type Damage%20Type%20Object%20Reference) (InstigatedBy :type Controller%20Object%20Reference) (DamageCauser :type Actor%20Object%20Reference))
  (Default|StartAction (Variables|Default|GetBPAC_TakingDamageAction) DamageCauser (Utilities|Array|MakeArray (Utilities|String|ToString(Float) Damage))))

(fn ConstructionScript)

(fn AttackPlayer
  (params (AttackingActor :type Actor%20Object%20Reference))
  (Default|StartAction (Variables|Default|GetBPAC_AttackingAction) AttackingActor (Utilities|Array|MakeArray (Utilities|String|ToString(Float) (Variables|AIConfig|GetEnemyDamage)))))

(fn PreparetoDeath
  (if (not (Variables|Default|GetIsDead))
    (Variables|AIConfig|SetIsAttacking false)
    (Default|StartAction (Variables|Default|GetBPAC_DeathAction) 0 (Utilities|Array|MakeArray ""))
    (Variables|Default|SetIsDead true)))

(fn CheckActorIsNear
  (params (Actor :type Actor%20Object%20Reference))
  (return (<= (Math|Vector|VectorLengthXY (- (Transformation|GetActorLocation Actor) (Transformation|GetActorLocation))) (+ (Variables|AIConfig|GetAttackRange) 0.0))))