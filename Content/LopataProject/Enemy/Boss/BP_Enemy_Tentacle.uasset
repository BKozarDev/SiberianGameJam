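; Boss tentacle enemy that rises in via a spawn timeline and attacks the player inside its box trigger.
; Overlap and Tick set IsAttacking; DamageDeal fires Niagara, enables capsule collision and calls AttackPlayer, while DisableDamamgeZone closes it and re-arms after a delay.
; A health component feeds a camera-facing health bar and has a zero-value event bound.
; The Attack timeline rotation logic is unwired; nothing here calls the damage events.
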(event OnComponentBeginOverlap(Box)
  (params (OverlappedComponent :type Primitive%20Component%20Object%20Reference) (OtherActor :type Actor%20Object%20Reference) (OtherComp :type Primitive%20Component%20Object%20Reference) (OtherBodyIndex :type Integer) (bFromSweep :type Boolean) (SweepResult :type Hit%20Result%20Structure%20%28by%20ref%29))
  (Utilities|Casting|CastToBP_PlayerChar OtherActor)
  (if (not (Variables|Default|GetIsAttacking))
    (if (not (Audio|Components|Audio|IsPlaying (Variables|Default|GetAttack)))
      (Variables|Default|SetIsAttacking true)
      (Variables|Default|SetPlayerInZone true))))

(event OnComponentEndOverlap(Box)
  (params (OverlappedComponent :type Primitive%20Component%20Object%20Reference) (OtherActor :type Actor%20Object%20Reference) (OtherComp :type Primitive%20Component%20Object%20Reference) (OtherBodyIndex :type Integer))
  (Utilities|Casting|CastToBP_PlayerChar OtherActor)
  (Variables|Default|SetPlayerInZone false)
  (Variables|Default|SetIsAttacking false))

(event Custom|DamageDeal
  (Components|Activation|Activate (Variables|Default|GetNiagara) false)
  (Collision|SetCollisionEnabled (Variables|Default|GetCapsule) "QueryOnly")
  (Variables|Default|SetPrepareAttack false)
  (if (Variables|Default|GetIsAttacking)
    (if (Variables|Default|GetPlayerInZone)
      (CallFunction|AttackPlayer (Game|GetPlayerCharacter 0)))
    (elif (Variables|Default|GetPlayerInZone)
      (Variables|Default|SetIsAttacking true))))

(event Custom|DisableDamamgeZone
  (Collision|SetCollisionEnabled (Variables|Default|GetCapsule) "NoCollision")
  (Utilities|FlowControl|Delay 0.65)
  (Variables|Default|SetPrepareAttack true))

(event EventBeginPlay
  (bind _aswbp_health_bar (Utilities|Casting|CastToWBP_HealthBar (UserInterface|GetUserWidgetObject (Variables|Default|GetWidgetHP))))
  (Default|SetupWidget _aswbp_health_bar (Variables|Default|GetBPAC_HealthComponent))
  (EventDispatchers|BindEventtoOnValueZero (Variables|Default|GetBPAC_HealthComponent) (EventDispatchers|CreateEvent :!event PreparetoDeath))
  (Rendering|SetCastShadow (Variables|Default|GetWidgetHP) false)
  (bind _offset (Timeline|TL_Spawn PlayFromStart)
    (:Update
      (Transformation|SetRelativeLocation (Variables|Character|GetMesh) (Math|Vector|MakeVector 0.0 0.0 _offset) false false))
    (:Finished
      (Variables|Default|SetPrepareAttack true))))

(event EventTick
  (params (DeltaSeconds :type Float%20%28single-precision%29))
  (Transformation|SetWorldRotation (Variables|Default|GetWidgetHP) (Math|Rotator|FindLookatRotation (Transformation|GetWorldLocation (Variables|Default|GetWidget)) (Camera|GetCameraLocation (Variables|/Script/Engine.PlayerController|GetPlayerCameraManager (Game|GetPlayerController 0)))) false false)
  (if (Variables|Default|GetPlayerInZone)
    (Variables|Default|SetIsAttacking (Variables|Default|GetPrepareAttack))))

(fn ConstructionScript
  (|CallParentFunction))