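; BP_Enemy_Tentacle is an enemy tentacle that swings at the player when they enter its box trigger.
; An Attack timeline pitches TentacleRoot, hits via AttackPlayer if the player is still in the zone, pauses, then reverses and repeats while they remain.
; A health component feeds a health bar widget, rotated each tick to face the camera, and has an event bound to zero health.
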(event OnComponentBeginOverlap(Box)
  (params (OverlappedComponent :type Primitive%20Component%20Object%20Reference) (OtherActor :type Actor%20Object%20Reference) (OtherComp :type Primitive%20Component%20Object%20Reference) (OtherBodyIndex :type Integer) (bFromSweep :type Boolean) (SweepResult :type Hit%20Result%20Structure%20%28by%20ref%29))
  (Utilities|Casting|CastToBP_PlayerChar OtherActor)
  (if (not (Variables|Default|GetIsAttacking))
    (if (not (Audio|Components|Audio|IsPlaying (Variables|Default|GetAttack)))
      (Variables|Default|SetIsAttacking true)
      (Audio|Components|Audio|Play (Variables|Default|GetAttack))
      (Variables|Default|SetPlayerInZone true))))

(event OnComponentEndOverlap(Box)
  (params (OverlappedComponent :type Primitive%20Component%20Object%20Reference) (OtherActor :type Actor%20Object%20Reference) (OtherComp :type Primitive%20Component%20Object%20Reference) (OtherBodyIndex :type Integer))
  (Utilities|Casting|CastToBP_PlayerChar OtherActor)
  (Variables|Default|SetPlayerInZone false))

(event EventBeginPlay
  (bind _aswbp_health_bar (Utilities|Casting|CastToWBP_HealthBar (UserInterface|GetUserWidgetObject (Variables|Default|GetWidgetHP))))
  (Default|SetupWidget _aswbp_health_bar (Variables|Default|GetBPAC_HealthComponent))
  (EventDispatchers|BindEventtoOnValueZero (Variables|Default|GetBPAC_HealthComponent) (EventDispatchers|CreateEvent :!event PreparetoDeath))
  (Rendering|SetCastShadow (Variables|Default|GetWidgetHP) false))

(event EventTick
  (params (DeltaSeconds :type Float%20%28single-precision%29))
  (Transformation|SetWorldRotation (Variables|Default|GetWidgetHP) (Math|Rotator|FindLookatRotation (Transformation|GetWorldLocation (Variables|Default|GetWidget)) (Camera|GetCameraLocation (Variables|/Script/Engine.PlayerController|GetPlayerCameraManager (Game|GetPlayerController 0)))) false false))

(fn ConstructionScript
  (|CallParentFunction))