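; BP_NotificationActor is a short-lived world-space notification that shows floating text through a widget component.
; On BeginPlay it passes its NotifText to the WBP_NotificationText widget, plays its animation, then destroys itself after a brief delay.
; Each tick it billboards the widget by rotating it to face the player camera.
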(event EventBeginPlay
  (bind _aswbp_notification_text (Utilities|Casting|CastToWBP_NotificationText (UserInterface|GetUserWidgetObject (Variables|Default|GetWidget))))
  (Default|SetupText _aswbp_notification_text (Variables|Default|GetNotifText))
  (Default|StartAnimation _aswbp_notification_text)
  (Utilities|FlowControl|Delay 1.0)
  (Actor|DestroyActor))

(event EventTick
  (params (DeltaSeconds :type Float%20%28single-precision%29))
  (Transformation|SetWorldRotation (Variables|Default|GetWidget) (Math|Rotator|FindLookatRotation (Transformation|GetWorldLocation (Variables|Default|GetWidget)) (Camera|GetCameraLocation (Variables|/Script/Engine.PlayerController|GetPlayerCameraManager (Game|GetPlayerController 0)))) false false))

(fn ConstructionScript)