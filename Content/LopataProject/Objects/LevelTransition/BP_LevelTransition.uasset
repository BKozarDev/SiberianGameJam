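; BP_LevelTransition is an interactable pit leading to the next level, previewing the reward class tied to it.
; On BeginPlay it registers with BP_LopataGameMode to obtain that class, then shows its icon on a camera-facing widget.
; When locked, interaction opens the pit by hiding the rock, playing effects and refreshing the prompt.
; When unlocked, it fires CallNextLevel with the reward, then unbinds and disables collision to prevent retriggering.
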(event EventTick
  (params (DeltaSeconds :type Float%20%28single-precision%29))
  (|CallParentFunction DeltaSeconds)
  (Transformation|SetWorldRotation (Variables|Default|GetRewardWidget) (Math|Rotator|FindLookatRotation (Transformation|GetWorldLocation (Variables|Default|GetRewardWidget)) (Camera|GetCameraLocation (Variables|/Script/Engine.PlayerController|GetPlayerCameraManager (Game|GetPlayerController 0)))) false false))

(event EventBeginPlay
  (|CallParentFunction)
  (bind _asbp_lopata_game_mode (Utilities|Casting|CastToBP_LopataGameMode (Game|GetGameMode)))
  (bind _rewardsclass (Default|BindTransition _asbp_lopata_game_mode self))
  (bind _output_get (Variables|Default|SetRewardClass _rewardsclass))
  (if (.ReturnValue (Utilities|Map|Find (Variables|Default|GetRewardClassIcons) _output_get))
    (bind _aswbp_pick_up_effect (Utilities|Casting|CastToWBP_PickUpEffect (UserInterface|GetUserWidgetObject (Variables|Default|GetRewardWidget))))
    (Default|SetupWidget _aswbp_pick_up_effect (.Value (Utilities|Map|Find (Variables|Default|GetRewardClassIcons) _output_get))))
  (if (Variables|Default|GetIsLocked)
    (Variables|/Game/LopataProject/Components/Actions/PlayerActions/BPAC_InteractionComponent.BPAC_InteractionComponent_C|SetInteractionText (Variables|Default|GetBPAC_InteractionComponent) (Variables|Default|GetLockedText))
    (else
      (Variables|/Game/LopataProject/Components/Actions/PlayerActions/BPAC_InteractionComponent.BPAC_InteractionComponent_C|SetInteractionText (Variables|Default|GetBPAC_InteractionComponent) (Variables|Default|GetUnlockedText)))))

(fn ConstructionScript
  (Rendering|SetVisibility (Variables|Default|GetRockMesh) (Variables|Default|GetIsLocked) false))

(fn ActivatePickUpEffect
  (params (TargetActor :type Actor%20Object%20Reference))
  (if (Variables|Default|GetIsLocked)
    (CallFunction|OpenPit)
    (Audio|PlaySound2D "/Game/LopataProject/Sounds/SC_OpenPit.SC_OpenPit" 1.0 1.0 0.0 0 0)
    (bind _success (Default|UpdateInfoinQueue (Variables|Default|GetBPAC_InteractionComponent) TargetActor))
    (return _success)
    (else
      (Default|CallCallNextLevel (Variables|Default|GetRewardClass))
      (EventDispatchers|UnbindallEventsfromCallNextLevel)
      (Collision|SetActorEnableCollision false)
      (return true))))

(fn OpenPit
  (Variables|Default|SetIsLocked false)
  (Rendering|SetVisibility (Variables|Default|GetRockMesh) false false)
  (Variables|/Game/LopataProject/Components/Actions/PlayerActions/BPAC_InteractionComponent.BPAC_InteractionComponent_C|SetInteractionText (Variables|Default|GetBPAC_InteractionComponent) (Variables|Default|GetUnlockedText))
  (Components|Activation|Activate (Variables|Default|GetOpenFX) false))