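; Health pickup actor that restores health to the actor that picks it up.
; ActivatePickUpEffect finds the target's BPAC_HealthComponent and, if health is not at maximum, increases it by IncreaseHealthValue and destroys the pickup.
; It returns whether the effect was applied, so the pickup stays in the world when the target has full health or no health component.
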(fn ConstructionScript
  (|CallParentFunction))

(fn ActivatePickUpEffect
  (params (TargetActor :type Actor%20Object%20Reference))
  (bind _output_get (LocalVariables|SetL_HealthComp (Actor|GetComponentbyClass TargetActor "/Game/LopataProject/Components/BPAC_HealthComponent.BPAC_HealthComponent_C")))
  (Utilities|IsValid _output_get
    (:Is%20Valid
      (if (== (Default|GetCurrentValue (LocalVariables|GetL_HealthComp)) (Default|GetMaxValue (LocalVariables|GetL_HealthComp)))
        (return false)
        (else
          (Default|IncreaseValue (LocalVariables|GetL_HealthComp) (Variables|Default|GetIncreaseHealthValue))
          (Actor|DestroyActor)
          (return true))))
    (:Is%20Not%20Valid
      (return false))))