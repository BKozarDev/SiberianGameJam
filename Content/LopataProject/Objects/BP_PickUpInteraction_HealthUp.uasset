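; Health-up pickup that raises the target actor's maximum and current health, then destroys itself.
; ActivatePickUpEffect finds the target's BPAC_HealthComponent, applies the truncated IncreaseValue to both values and returns whether it succeeded.
; On BeginPlay it sets up a WBP_PickUpEffect widget with its icon, and each Tick rotates that widget component to face the player camera.
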(event EventBeginPlay
  (bind _aswbp_pick_up_effect (Utilities|Casting|CastToWBP_PickUpEffect (UserInterface|GetUserWidgetObject (Variables|Default|GetWidget))))
  (Variables|Default|SetWidgetEffect _aswbp_pick_up_effect)
  (Default|SetupWidget _aswbp_pick_up_effect (Variables|Default|GetSetup%20Icon)))

(event EventTick
  (params (DeltaSeconds :type Float%20%28single-precision%29))
  (Transformation|SetWorldRotation (Variables|Default|GetWidget) (Math|Rotator|FindLookatRotation (Transformation|GetWorldLocation (Variables|Default|GetWidget)) (Camera|GetCameraLocation (Variables|/Script/Engine.PlayerController|GetPlayerCameraManager (Game|GetPlayerController 0)))) false false))

(fn ConstructionScript
  (|CallParentFunction))

(fn ActivatePickUpEffect
  (params (TargetActor :type Actor%20Object%20Reference))
  (bind _increasevalue (Variables|Default|GetIncreaseValue))
  (bind _returnvalue (Math|Float|Truncate _increasevalue))
  (bind _output_get (LocalVariables|SetL_HealthComp (Actor|GetComponentbyClass TargetActor "/Game/LopataProject/Components/BPAC_HealthComponent.BPAC_HealthComponent_C")))
  (Utilities|IsValid _output_get
    (:Is%20Valid
      (Default|IncreaseMaxValue (LocalVariables|GetL_HealthComp) _returnvalue)
      (Default|IncreaseValue (LocalVariables|GetL_HealthComp) _returnvalue)
      (Actor|DestroyActor)
      (return true))
    (:Is%20Not%20Valid
      (return false))))