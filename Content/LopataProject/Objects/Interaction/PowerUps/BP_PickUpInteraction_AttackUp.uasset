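; An attack power-up pickup that raises the player's attack by a configurable increase value.
; Its ActivatePickUpEffect applies the increase only to a BP_PlayerChar target, returning false for any other actor.
; On success it spawns a notification actor showing the bonus as a damage percentage in Russian, plays a pickup sound, signals that it was picked up and destroys itself.
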(fn ConstructionScript
  (|CallParentFunction))

(fn ActivatePickUpEffect
  (params (TargetActor :type Actor%20Object%20Reference))
  (bind _increasevalue (Variables|Default|GetIncreaseValue))
  (bind _asbp_player_char (Utilities|Casting|CastToBP_PlayerChar TargetActor)
    (:then
      (Default|IncreaseAttack _asbp_player_char _increasevalue)
      (Game|SpawnActorfromClass "/Game/LopataProject/Objects/BP_NotificationActor.BP_NotificationActor_C" (Transformation|GetActorTransform) "Undefined" "MultiplyWithRoot" 0 (Utilities|Text|FormatText "+{Value}%Урона" (* _increasevalue 1e+02)) 0)
      (Audio|PlaySound2D "/Game/LopataProject/Sounds/SC_PickUp.SC_PickUp" 1.0 1.0 0.0 0 0)
      (Default|CallOnPickedUp)
      (Actor|DestroyActor)
      (return true))
    (:CastFailed
      (return false))))