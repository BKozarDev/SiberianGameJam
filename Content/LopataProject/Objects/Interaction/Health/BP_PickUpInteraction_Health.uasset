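; BP_PickUpInteraction_Health is a health pickup that heals the target actor through its BPAC_HealthComponent.
; ActivatePickUpEffect refuses if that component is missing or full; otherwise it raises health, spawns a healing notification actor, plays a sound and destroys the pickup.
; BeginPlay sets up the icon widget and disables its shadow.
; Tick turns the widget toward the player camera and spins the mesh by a fixed, frame-rate-dependent step.
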(event EventBeginPlay
  (bind _aswbp_pick_up_effect (Utilities|Casting|CastToWBP_PickUpEffect (UserInterface|GetUserWidgetObject (Variables|Default|GetWidget))))
  (Variables|Default|SetWidgetEffect _aswbp_pick_up_effect)
  (Default|SetupWidget _aswbp_pick_up_effect (Variables|Default|GetSetup%20Icon))
  (Rendering|SetCastShadow (Variables|Default|GetWidget) false))

(event EventTick
  (params (DeltaSeconds :type Float%20%28single-precision%29))
  (Transformation|SetWorldRotation (Variables|Default|GetWidget) (Math|Rotator|FindLookatRotation (Transformation|GetWorldLocation (Variables|Default|GetWidget)) (Camera|GetCameraLocation (Variables|/Script/Engine.PlayerController|GetPlayerCameraManager (Game|GetPlayerController 0)))) false false)
  (Transformation|AddWorldRotation (Variables|Default|GetPickUpMesh) (Math|Rotator|MakeRotator 0.0 0.0 2.0) false false))

(fn ConstructionScript
  (|CallParentFunction))

(fn ActivatePickUpEffect
  (params (TargetActor :type Actor%20Object%20Reference))
  (bind _output_get (LocalVariables|SetL_HealthComp (Actor|GetComponentbyClass TargetActor "/Game/LopataProject/Components/BPAC_HealthComponent.BPAC_HealthComponent_C")))
  (Utilities|IsValid _output_get
    (:Is%20Valid
      (if (== (Default|GetCurrentValue (LocalVariables|GetL_HealthComp)) (Default|GetMaxValue (LocalVariables|GetL_HealthComp)))
        (return false)
        (else
          (Default|IncreaseValue (LocalVariables|GetL_HealthComp) (Variables|Default|GetIncreaseHealthValue))
          (Game|SpawnActorfromClass "/Game/LopataProject/Objects/BP_NotificationActor.BP_NotificationActor_C" (Transformation|GetActorTransform) "Undefined" "MultiplyWithRoot" 0 (Utilities|Text|FormatText "++Лечение") 0)
          (Audio|PlaySound2D "/Game/LopataProject/Sounds/SC_PickUp.SC_PickUp" 1.0 1.0 0.0 0 0)
          (Actor|DestroyActor)
          (return true))))
    (:Is%20Not%20Valid
      (return false))))