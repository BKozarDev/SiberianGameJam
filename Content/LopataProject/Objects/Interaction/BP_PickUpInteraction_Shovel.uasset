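; Shovel pickup interaction actor that spins its mesh in the world until the player collects it.
; Tick adds a fixed yaw step to PickUpMesh each frame, without delta-time scaling.
; ActivatePickUpEffect accepts only BP_PlayerChar, then plays the SC_OpenPit sound, fires OnPickedUp and destroys the actor.
; It grants nothing to the player directly, leaving any follow-up to whatever handles OnPickedUp.
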(event EventBeginPlay
  (|CallParentFunction) ; This node is disabled and will not be called.\nDrag off pins to build functionality.
)

(event EventTick
  (params (DeltaSeconds :type Float%20%28single-precision%29))
  (Transformation|AddWorldRotation (Variables|Default|GetPickUpMesh) (Math|Rotator|MakeRotator 0.0 0.0 2.0) false false))

(fn ConstructionScript
  (|CallParentFunction))

(fn ActivatePickUpEffect
  (params (TargetActor :type Actor%20Object%20Reference))
  (Utilities|Casting|CastToBP_PlayerChar TargetActor)
  (Audio|PlaySound2D "/Game/LopataProject/Sounds/SC_OpenPit.SC_OpenPit" 1.0 1.0 0.0 0 0)
  (Default|CallOnPickedUp)
  (Actor|DestroyActor)
  (return false))