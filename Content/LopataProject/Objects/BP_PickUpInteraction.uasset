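; Pickup actor that is collected through an interaction system when an interactor starts an interaction with it.
; Overlaps on its ActivationTrigger add or remove the other actor from the queue of its BPAC interaction component.
; StartInteraction passes the interactor to ActivatePickUp, which is defined outside these graphs, and returns its result.
; Interact and StopInteraction only return false, and the construction script just calls the parent's.
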(event OnComponentBeginOverlap(ActivationTrigger)
  (params (OverlappedComponent :type Primitive%20Component%20Object%20Reference) (OtherActor :type Actor%20Object%20Reference) (OtherComp :type Primitive%20Component%20Object%20Reference) (OtherBodyIndex :type Integer) (bFromSweep :type Boolean) (SweepResult :type Hit%20Result%20Structure%20%28by%20ref%29))
  (bind _success (Default|AddtoQueue (Variables|Default|GetBPAC_InteractionComponent) OtherActor))
  (if _success
    _))

(event OnComponentEndOverlap(ActivationTrigger)
  (params (OverlappedComponent :type Primitive%20Component%20Object%20Reference) (OtherActor :type Actor%20Object%20Reference) (OtherComp :type Primitive%20Component%20Object%20Reference) (OtherBodyIndex :type Integer))
  (bind _success (Default|RemovefromQueue (Variables|Default|GetBPAC_InteractionComponent) OtherActor))
  (if _success
    _))

(fn ConstructionScript
  (|CallParentFunction))

(fn Interact
  (params (Interactor :type Actor%20Object%20Reference))
  (return false))

(fn Startinteraction
  (params (Interactor :type Actor%20Object%20Reference))
  (bind _success (CallFunction|ActivatePickUp Interactor))
  (return _success))

(fn StopInteraction
  (params (Interactor :type Actor%20Object%20Reference))
  (return false))