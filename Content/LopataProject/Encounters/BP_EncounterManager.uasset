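; BP_EncounterManager runs a sequence of encounters from BeginPlay, each with optional start and end delays.
; It shows Niagara spawn effects at random reachable navmesh points near the world origin, then spawns the encounter's enemies there after a short wait.
; Each enemy's death component event decrements a counter.
; When it empties, or if the encounter has no enemies, rewards spawn at random points and the sequence advances.
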(event Custom|NextEncounter
  (bind _encounters (Variables|EncounterManager|GetEncounters))
  (bind _result (Math|Integer|IncrementInt (Variables|Default|GetCurrentEncounterIdx))
    (:%20%20
      (if (Utilities|Array|IsValidIndex _encounters _result)
        (Variables|Default|SetCurrentEncounter (Utilities|Array|Get(acopy) _encounters (Variables|Default|GetCurrentEncounterIdx)))
        (if (> (.StartDelay (Utilities|Struct|BreakEncounterData (Variables|Default|GetCurrentEncounter))) 0.0)
          (bind _returnvalue (Utilities|Time|SetTimerbyEvent (delegate Custom|StartDelayComplete) (.StartDelay (Utilities|Struct|BreakEncounterData (Variables|Default|GetCurrentEncounter)))))
          (Variables|Default|SetTimersHandle _returnvalue)
          (else
            (CallFunction|StartDelayComplete)))))))

(event Custom|EnemyDied
  (params (DiedActor :type Actor%20Object%20Reference))
  (bind _result (Math|Integer|DecrementInt (Variables|Default|GetEnemiesCounter))
    (:%20%20
      (if (<= _result 0)
        (CallFunction|SpawnRewards)))))

(event Custom|SpawnEnemies
  (bind _spawnlocs (Variables|Default|GetSpawnLocs))
  (Variables|Default|SetEnemiesCounter 0)
  (Utilities|Array|Clear (Variables|Default|GetSpawnLocs))
  (for _array_element (Utilities|Struct|BreakEncounterData (Variables|Default|GetCurrentEncounter))
    (bind _returnvalue (Utilities|Array|Add _spawnlocs (+ (.RandomLocation (AI|Navigation|GetRandomReachablePointinRadius (Math|Vector|MakeVector 0.0 0.0 1e+01) 1.5e+03 0 0)) "0.000000,0.000000,100.000000")))
    (Niagara|SpawnSystematLocation "/Game/LopataProject/Common/FX/NS_EnemySpawnEffect.NS_EnemySpawnEffect" (+ (Utilities|Array|Get(acopy) _spawnlocs _returnvalue) "0.000000,0.000000,-100.000000")))
  (Utilities|FlowControl|Delay 1.35)
  (for (_array_element_2 _array_index) (Utilities|Struct|BreakEncounterData (Variables|Default|GetCurrentEncounter))
    (bind _returnvalue_2 (Game|SpawnActorfromClass _array_element_2 (Math|Transform|MakeTransform (Utilities|Array|Get(acopy) (Variables|Default|GetSpawnLocs) _array_index) "0, 0, 0" "1.000000,1.000000,1.000000") "AdjustIfPossibleButAlwaysSpawn" "MultiplyWithRoot" 0 0))
    (EventDispatchers|BindEventtoOwnerDied (Variables|/Game/LopataProject/Enemy/BP_EnemyBase.BP_EnemyBase_C|GetBPAC_DeathAction _returnvalue_2) (delegate Custom|EnemyDied))
    (Math|Integer|IncrementInt (Variables|Default|GetEnemiesCounter))))

(event Custom|SpawnRewards
  (bind _currentencounter (Variables|Default|GetCurrentEncounter))
  (bind (_rewardslist _enddelay) (Utilities|Struct|BreakEncounterData _currentencounter))
  (for _array_element _rewardslist
    (Game|SpawnActorfromClass _array_element (Math|Transform|MakeTransform (+ (.RandomLocation (AI|Navigation|GetRandomReachablePointinRadius (Math|Vector|MakeVector 0.0 0.0 1e+01) 1.5e+03 0 0)) "0.000000,0.000000,100.000000") "0, 0, 0" "1.000000,1.000000,1.000000") "AdjustIfPossibleButAlwaysSpawn" "MultiplyWithRoot" 0 0))
  (if (> _enddelay 0.0)
    (bind _returnvalue (Utilities|Time|SetTimerbyEvent (EventDispatchers|CreateEvent :!event Custom|NextEncounter) _enddelay))
    (Variables|Default|SetTimersHandle _returnvalue)
    (else
      (CallFunction|NextEncounter))))

(event Custom|StartDelayComplete
  (if (Utilities|Array|IsNotEmpty (.EnemiesList (Utilities|Struct|BreakEncounterData (Variables|Default|GetCurrentEncounter))))
    (CallFunction|SpawnEnemies)
    (else
      (CallFunction|SpawnRewards))))

(event EventBeginPlay
  (Variables|Default|SetCurrentEncounterIdx -1)
  (CallFunction|NextEncounter))

(fn ConstructionScript)